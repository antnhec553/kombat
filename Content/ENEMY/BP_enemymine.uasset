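; BP_enemymine is an enemy character that chases the player and attacks in melee.
; PawnSensing starts the chase via AIMoveTo; on arrival it plays a combo montage and damages players in a sphere at Point, gated by CanAttack until the montage duration elapses.
; AnyDamage lowers Health and prints while it stays positive, with no death handling.
; The AIPerception handler only casts, and CanSeePawn is never cleared.
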(event `chase`
  (if (`self.can see pawn`)
    (`|AIMoveTo` self (0.0 0.0 0.0) (`GameplayStatics.GetPlayerCharacter` 0)
      (:`OnSuccess`
        (if (`self.can attack`)
          (set `self.can attack` false)
          (bind _returnvalue (`self.PlayAnimMontage` "/Game/ENEMY/AM-enemyattackcombo.AM-enemyattackcombo"))
          (bind _outactors (`KismetSystemLibrary.SphereOverlapActors` (`SceneComponent.K2_GetComponentLocation` (`self.point`)) 100.0 (`self.Object Types`) "/Game/ThirdPerson/Blueprints/BP_ThirdPersonCharacter.BP_ThirdPersonCharacter_C"))
          (for _array_element _outactors
            (`GameplayStatics.ApplyDamage` _array_element 10.0))
          (`KismetSystemLibrary.Delay` _returnvalue)
          (set `self.can attack` true))))))

(event `self.PawnSensing.OnSeePawn`
  (params (Pawn :type "Pawn Object Reference"))
  (set `self.can see pawn` true)
  (`self.chase`))

(event `self.ReceiveAnyDamage`
  (params (Damage :type "Float (single-precision)") (DamageType :type "DamageType Object Reference") (InstigatedBy :type "Controller Object Reference") (DamageCauser :type "Actor Object Reference"))
  (set `self.health` (- (`self.health`) Damage))
  (if (> (`self.health`) 0.0)
    (`KismetSystemLibrary.PrintString` "damage")))

(event `self.AIPerception.OnTargetPerceptionUpdated`
  (params (Actor :type "Actor Object Reference") (Stimulus :type "AIStimulus Structure"))
  (cast `/Game/ThirdPerson/Blueprints/BP_ThirdPersonCharacter` Actor))

(fn `UserConstructionScript`)